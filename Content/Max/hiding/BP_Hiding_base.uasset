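; BP_Hiding_base is a base hiding-spot actor that marks the player as hidden while they stand inside its box volume.
; BoxCollision_hiding overlap events check for the "Player" tag, then cast player character 0 to BP_Character_Fabe.
; They set its IsHiding flag true on entering and false on leaving; the construction script is empty.
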(event OnComponentBeginOverlap(BoxCollision_hiding)
  (params (OverlappedComponent :type Primitive%20Component%20Object%20Reference) (OtherActor :type Actor%20Object%20Reference) (OtherComp :type Primitive%20Component%20Object%20Reference) (OtherBodyIndex :type Integer) (bFromSweep :type Boolean) (SweepResult :type Hit%20Result%20Structure%20%28by%20ref%29))
  (if (Actor|ActorHasTag OtherActor "Player")
    (bind _asbp_character_fabe (Utilities|Casting|CastToBP_Character_Fabe (Game|GetPlayerCharacter 0)))
    (Variables|/Game/Fabian/Blueprints/BP_Character_Fabe.BP_Character_Fabe_C|SetisHiding? _asbp_character_fabe true)))

(event OnComponentEndOverlap(BoxCollision_hiding)
  (params (OverlappedComponent :type Primitive%20Component%20Object%20Reference) (OtherActor :type Actor%20Object%20Reference) (OtherComp :type Primitive%20Component%20Object%20Reference) (OtherBodyIndex :type Integer))
  (if (Actor|ActorHasTag OtherActor "Player")
    (bind _asbp_character_fabe (Utilities|Casting|CastToBP_Character_Fabe (Game|GetPlayerCharacter 0)))
    (Variables|/Game/Fabian/Blueprints/BP_Character_Fabe.BP_Character_Fabe_C|SetisHiding? _asbp_character_fabe false)))

(fn ConstructionScript)