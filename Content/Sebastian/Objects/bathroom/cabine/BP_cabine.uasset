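; Interactable bathroom cabinet whose door swings open or closed when a player interacts with it.
; InteractFunction runs the parent interaction, then calls Open Cabinet, which toggles the door-open flag.
; A timeline plays from the start to open and reverses to close, driving the yaw of the door pivot.
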(event Custom|Open_Cabinet
  (if (Variables|Default|GetIsCabineDoorOpen)
    (Variables|Default|SetIsCabineDoorOpen false)
    (bind _doorfloat (Timeline|OpenDoorTimeline Reverse)
      (:Update
        (Transformation|SetRelativeRotation (Variables|Default|GetPivot_door) (Math|Rotator|MakeRotator 0.0 0.0 _doorfloat) false false)))
    (else
      (Variables|Default|SetIsCabineDoorOpen true)
      (Timeline|OpenDoorTimeline PlayFromStart))))

(fn ConstructionScript)

(fn InteractFunction
  (params (PlayerRef :type BP%20Character%20Fabe%20Object%20Reference))
  (|CallParentFunction PlayerRef)
  (CallFunction|OpenCabinet))