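; BP_door_hallway is a hallway door Blueprint whose opening logic is disconnected and does not move the door as wired.
; OpenDoor has a constant branch that skips the door sound and a dot-product test of which side the player stands on, which leads nowhere.
; An unreachable timeline would set relative yaw, but its lerp endpoints are both zero, and its finish sound sits behind another constant branch.
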(event Custom|Open%20Door
  (if (not true)
    (Audio|SpawnSoundAttached "/Game/Almin/character/door/door_sound.door_sound" 0 "None" "0, 0, 0" "0, 0, 0" "KeepRelativeOffset" false 1.0 1.0 0.0 0 0)
    (if (> (Math|Vector|DotProduct (Math|Vector|Normalize (- (Transformation|GetActorLocation (Game|GetPlayerCharacter 0)) (Transformation|GetActorLocation))) (Transformation|GetActorRightVector)) 0.0)
      _)))

(fn ConstructionScript)