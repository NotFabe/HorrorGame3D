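; Interactable keycard scanner that opens its double doors when the player holds the required colour keycard, and otherwise plays a decline sound and HUD message.
; A timeline swings the doors while dynamic materials switch the light from red to green.
; Green and blue cards also open any linked elevator door.
; Red triggers the win screen and pauses the game; orange halts the enemy AI and teleports the enemy to a spawn point.
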(event Custom|OpenDoor
  (bind _doorangle (Timeline|TL_OpenDoor Play)
    (:Update
      (Transformation|SetRelativeRotation (Variables|Default|GetPivotLeftDoor) (Math|Rotator|MakeRotator 0.0 0.0 (- 9e+01 _doorangle)) false false)
      (Transformation|SetRelativeRotation (Variables|Default|GetPivotRightDoor) (Math|Rotator|MakeRotator 0.0 0.0 (+ _doorangle 9e+01)) false false)
      (Collision|SetCollisionResponsetoChannel (Variables|Default|GetScanner) "ECC_Visibility" "ECR_Ignore")
      (Rendering|Material|SetScalarParameterValue (Variables|Default|GetRedMat) "Brightness" 0.0 :!class /Script/Engine.MaterialInstanceDynamic)
      (Rendering|Material|SetScalarParameterValue (Variables|Default|GetGreenMat) "Brightness" 1e+01 :!class /Script/Engine.MaterialInstanceDynamic))))

(event Custom|EndGame
  (bind _returnvalue (Game|GetPlayerController 0))
  (bind _returnvalue_2 (UserInterface|CreateWidget "/Game/Max/winscreen/WB_WinScreen.WB_WinScreen_C"))
  (UserInterface|Viewport|AddtoViewport _returnvalue_2 0)
  (Audio|PlaySoundatLocation "/Game/Almin/türen/keycard/keycard_accept_bearbeitet.keycard_accept_bearbeitet" "0, 0, 0" "0, 0, 0" 1.0 1.0 0.0 0 0 0 0)
  (CallFunction|OpenDoor)
  (Utilities|FlowControl|Delay 0.7)
  (Audio|PlaySound2D "/Game/Max/winscreen/gamewinsound.gamewinsound" 1.0 1.0 0.0 0 0)
  (Utilities|FlowControl|Delay 0.7)
  (Game|SetGamePaused true)
  (Input|SetInputModeGameandUI _returnvalue 0 "DoNotLock" false false)
  (Variables|/Script/Engine.PlayerController|SetbShowMouseCursor _returnvalue true))

(event EventBeginPlay
  (bind _returnvalue (Rendering|Material|CreateDynamicMaterialInstance (Variables|Default|GetRedlight) 0 0 "None" :!class /Script/Engine.PrimitiveComponent))
  (Variables|Default|SetRedMat _returnvalue)
  (bind _returnvalue_2 (Rendering|Material|CreateDynamicMaterialInstance (Variables|Default|GetGreenlight) 0 0 "None" :!class /Script/Engine.PrimitiveComponent))
  (Variables|Default|SetGreenMat _returnvalue_2)
  (Rendering|Material|SetScalarParameterValue (Variables|Default|GetRedMat) "Brightness" 1e+01 :!class /Script/Engine.MaterialInstanceDynamic)
  (Rendering|Material|SetScalarParameterValue (Variables|Default|GetGreenMat) "Brightness" 0.0 :!class /Script/Engine.MaterialInstanceDynamic))

(fn ConstructionScript
  (Rendering|Material|SetMaterial (Variables|Default|GetScannerIcon) 0 (Variables|Default|GetKeycardTextureColour))
  (Variables|Default|SetHighlightMesh (Variables|Default|GetScanner)))

(fn InteractFunction
  (params (PlayerRef :type BP%20Character%20Fabe%20Object%20Reference))
  (bind _requieredkeycard (Variables|Default|GetRequieredKeycard))
  (bind _elevatordoorref (Variables|Default|GetElevatorDoorRef))
  (|CallParentFunction PlayerRef)
  (switch Utilities|FlowControl|Switch|SwitchonEnum_KeycardColour _requieredkeycard
    (:NewEnumerator0
      (if (Variables|/Game/Fabian/Blueprints/BP_Character_Fabe.BP_Character_Fabe_C|GetHasKeyCardGreen PlayerRef)
        (Audio|PlaySoundatLocation "/Game/Almin/türen/keycard/keycard_accept_bearbeitet.keycard_accept_bearbeitet" "0, 0, 0" "0, 0, 0" 1.0 1.0 0.0 0 0 0 0 :!label _label)
        (CallFunction|OpenDoor)
        (Utilities|IsValid _elevatordoorref
          (:Is%20Valid
            (Default|OpenElevatorDoor _elevatordoorref)))
        (else
          (Audio|PlaySoundatLocation "/Game/Almin/türen/keycard/keycard_decline_bearbeitet.keycard_decline_bearbeitet" "0, 0, 0" "0, 0, 0" 1.0 1.0 0.0 0 0 0 0 :!label _label_2)
          (Default|PlayMissingCardText (Variables|/Game/Fabian/Blueprints/BP_Character_Fabe.BP_Character_Fabe_C|GetHUDWidget PlayerRef) (Utilities|Text|ToText(String) (Utilities|String|EnumtoString _requieredkeycard))))))
    (:NewEnumerator6
      (if (Variables|/Game/Fabian/Blueprints/BP_Character_Fabe.BP_Character_Fabe_C|GetHasKeyCardRed PlayerRef)
        (CallFunction|EndGame)
        (else
          (goto _label_2))))
    (:NewEnumerator7
      (if (Variables|/Game/Fabian/Blueprints/BP_Character_Fabe.BP_Character_Fabe_C|GetHasKeyCardBlue PlayerRef)
        (goto _label)
        (else
          (goto _label_2))))
    (:NewEnumerator8
      (if (Variables|/Game/Fabian/Blueprints/BP_Character_Fabe.BP_Character_Fabe_C|GetHasKeyCardOrange PlayerRef)
        (Audio|PlaySoundatLocation "/Game/Almin/türen/keycard/keycard_accept_bearbeitet.keycard_accept_bearbeitet" "0, 0, 0" "0, 0, 0" 1.0 1.0 0.0 0 0 0 0)
        (CallFunction|OpenDoor)
        (bind _returnvalue (Actor|GetActorOfClass "/Game/Max/enemy/enemy_char.enemy_char_C"))
        (bind _returnvalue_2 (Actor|GetActorOfClass "/Game/Max/enemy/ai_controller_max.ai_controller_max_C"))
        (AI|Navigation|StopMovement _returnvalue_2)
        (AI|ClearFocus _returnvalue_2)
        (Transformation|Teleport _returnvalue (Transformation|GetActorLocation (Variables|Default|GetspawnPointenemy)) "0, 0, 0")
        (else
          (goto _label_2))))))