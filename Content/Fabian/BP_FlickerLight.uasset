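; BP_FlickerLight is a light fixture actor that flickers at random during play.
; On BeginPlay it creates a dynamic instance of M_LightFlickMat on the static mesh's second material slot, then starts the Flickering event.
; Flickering sets a random RectLight intensity, drives the material's GlowStrength from the same value so glow and light match, then calls itself again after a short random delay.
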(event Custom|Flickering
  (Variables|Default|SetRandomLightInten (Math|Random|RandomFloatinRange 0.0 1e+03))
  (Rendering|Components|Light|SetIntensity (Variables|Default|GetRectLight) (Variables|Default|GetRandomLightInten))
  (Rendering|Material|SetScalarParameterValue (Variables|Default|GetDynamicMat) "GlowStrength" (/ (Variables|Default|GetRandomLightInten) 25.0) :!class /Script/Engine.MaterialInstanceDynamic)
  (Utilities|FlowControl|Delay (Math|Random|RandomFloatinRange 0.01 0.2))
  (CallFunction|Flickering))

(event EventBeginPlay
  (bind _returnvalue (Rendering|Material|CreateDynamicMaterialInstance (Variables|Default|GetStaticMesh) 1 "/Game/Fabian/M_LightFlickMat.M_LightFlickMat" "None" :!class /Script/Engine.PrimitiveComponent))
  (bind _output_get (Variables|Default|SetDynamicMat _returnvalue))
  (Rendering|Material|SetMaterial (Variables|Default|GetStaticMesh) 1 _output_get)
  (CallFunction|Flickering))

(fn ConstructionScript)