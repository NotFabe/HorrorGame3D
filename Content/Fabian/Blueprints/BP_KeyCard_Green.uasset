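; Green keycard pickup that grants the player access via a green keycard flag.
; Construction sets the Keycard mesh as the parent's highlight mesh.
; On interact it runs the parent interaction, shows a HUD pickup text built from its colour enum plus "KEYCARD", sets HasKeyCardGreen on the player, then destroys itself.
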(fn ConstructionScript
  (Variables|Default|SetHighlightMesh (Variables|Default|GetKeycard)))

(fn InteractFunction
  (params (PlayerRef :type BP%20Character%20Fabe%20Object%20Reference))
  (|CallParentFunction PlayerRef)
  (Default|PlayPickupText (Variables|/Game/Fabian/Blueprints/BP_Character_Fabe.BP_Character_Fabe_C|GetHUDWidget PlayerRef) (Utilities|Text|ToText(String) (Utilities|String|Append (Utilities|String|EnumtoString (Variables|Default|GetColour)) " KEYCARD")))
  (Variables|/Game/Fabian/Blueprints/BP_Character_Fabe.BP_Character_Fabe_C|SetHasKeyCardGreen PlayerRef true)
  (Actor|DestroyActor))