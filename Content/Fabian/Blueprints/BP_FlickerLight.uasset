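; BP_FlickerLight is a ceiling light that flickers endlessly at random, with occasional lamp noise.
; On BeginPlay it puts a dynamic material instance on the fixture mesh, then starts a self-calling Flickering event with short random delays.
; Each pass randomizes the RectLight intensity, scales the material's GlowStrength to match, and occasionally plays the sound at world origin rather than at the lamp.
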(event Custom|Flickering
  (Variables|Default|SetRandomLightInten (Math|Random|RandomFloatinRange 25.0 4e+02))
  (Rendering|Components|Light|SetIntensity (Variables|Default|GetRectLight) (Variables|Default|GetRandomLightInten))
  (Rendering|Material|SetScalarParameterValue (Variables|Default|GetDynamicMat) "GlowStrength" (/ (Variables|Default|GetRandomLightInten) 25.0) :!class /Script/Engine.MaterialInstanceDynamic)
  (if (Math|Random|RandomBoolwithWeight 0.2)
    (Audio|PlaySoundatLocation "/Game/Almin/ambience/base_ambience/lampen_geraeucshe_original.lampen_geraeucshe_original" "0, 0, 0" "0, 0, 0" 1.0 1.0 0.0 0 0 0 0))
  (Utilities|FlowControl|Delay (Math|Random|RandomFloatinRange 0.01 0.2))
  (CallFunction|Flickering))

(event EventBeginPlay
  (bind _theappxr_luce_soffitto_1_nodraco_standard (Variables|Default|Gettheappxr_Luce_Soffitto_1_NODRACO_standard))
  (bind _returnvalue (Rendering|Material|CreateDynamicMaterialInstance _theappxr_luce_soffitto_1_nodraco_standard 1 "/Game/Fabian/Materials/M_LightFlickMat.M_LightFlickMat" "None" :!class /Script/Engine.PrimitiveComponent))
  (bind _output_get (Variables|Default|SetDynamicMat _returnvalue))
  (Rendering|Material|SetMaterial _theappxr_luce_soffitto_1_nodraco_standard 1 _output_get)
  (CallFunction|Flickering))

(fn ConstructionScript)