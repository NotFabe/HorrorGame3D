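; BP_VentCover is an interactable vent cover that swings open when the player uses it.
; The construction script assigns the vent mesh as the parent class's highlight mesh, and the interact override calls the parent before triggering OpenVent.
; OpenVent plays a metal sound and a timeline that pitches the pivot, then sets the mesh to ignore the Visibility channel once finished.
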(event Custom|OpenVent
  (Audio|PlaySoundatLocation "/Game/Fabian/Sounds/Metal_Vent_Open.Metal_Vent_Open" (Transformation|GetWorldLocation (Variables|Default|GetVentMesh)) "0, 0, 0" 1.0 1.0 0.0 0 0 0 0)
  (bind _ventrotation (Timeline|Timeline Play)
    (:Update
      (Transformation|SetRelativeRotation (Variables|Default|GetVentPivot) (Math|Rotator|MakeRotator 0.0 (* _ventrotation -1.0) 0.0) false false))
    (:Finished
      (Collision|SetCollisionResponsetoChannel (Variables|Default|GetVentMesh) "ECC_Visibility" "ECR_Ignore"))))

(fn ConstructionScript
  (|CallParentFunction)
  (Variables|Default|SetHighlightMesh (Variables|Default|GetVentMesh)))

(fn InteractFunction
  (params (PlayerRef :type BP%20Character%20Fabe%20Object%20Reference))
  (|CallParentFunction PlayerRef)
  (CallFunction|OpenVent))